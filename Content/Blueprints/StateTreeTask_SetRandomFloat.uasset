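; StateTree task that writes a random float between configurable minimum and maximum values to an output value.
; The roll happens on state entry only when the transition's change type is Changed, so sustained states keep their value.
; The task never calls Finish Task.
; A description override shows the configured range as a formatted summary.
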(event `self.ReceiveLatentEnterState`
  (params (Transition :type "StateTreeTransitionResult Structure (by ref)"))
  (if (`|EnumEquality` (`.ChangeType` (break `StateTreeTransitionResult` Transition)) "Changed")
    (set `self.Out Value` (`KismetMathLibrary.RandomFloatInRange` (`self.Min Value`) (`self.Max Value`)))))

(fn `ReceiveGetDescription`
  (params (Formatting :type "EStateTreeNodeFormatting Enum" :default "RichText"))
  (returns (ReturnValue :type Text))
  (return (`|FormatText` "Calculate random float between {min} and {max} on Enter" (`self.Min Value`) (`self.Max Value`))))
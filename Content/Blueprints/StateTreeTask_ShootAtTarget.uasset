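; A StateTree task that makes a character shoot at a target for as long as its state is active.
; On a changed transition, entering the state calls StartShooting on the Character with the Target, and exiting calls StopShooting.
; The task never finishes itself, and it supplies an editor description stating that behavior.
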(event `self.ReceiveLatentEnterState`
  (params (Transition :type "StateTreeTransitionResult Structure (by ref)"))
  (if (`|EnumEquality` (`.ChangeType` (break `StateTreeTransitionResult` Transition)) "Changed")
    (`/Game/Blueprints/BP_ShooterNPC.Start Shooting` (`self.Character`) (`self.Target`))))

(event `self.ReceiveExitState`
  (params (Transition :type "StateTreeTransitionResult Structure (by ref)"))
  (if (`|EnumEquality` (`.ChangeType` (break `StateTreeTransitionResult` Transition)) "Changed")
    (`/Game/Blueprints/BP_ShooterNPC.Stop Shooting` (`self.Character`))))

(fn `ReceiveGetDescription`
  (params (Formatting :type "EStateTreeNodeFormatting Enum" :default "RichText"))
  (returns (ReturnValue :type Text))
  (return "Shoot at Target while State is Active"))
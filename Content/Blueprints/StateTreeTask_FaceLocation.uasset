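; StateTree task that makes an AI controller face a target location while its state is active.
; Entering the state through a changed transition sets the controller's focal point to TargetLocation.
; Exiting through a changed transition clears the focus, while sustained transitions leave it untouched.
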(event `self.ReceiveLatentEnterState`
  (params (Transition :type "StateTreeTransitionResult Structure (by ref)"))
  (if (`|EnumEquality` (`.ChangeType` (break `StateTreeTransitionResult` Transition)) "Changed")
    (`AIController.K2_SetFocalPoint` (`self.Controller`) (`self.Target Location`))))

(event `self.ReceiveExitState`
  (params (Transition :type "StateTreeTransitionResult Structure (by ref)"))
  (if (`|EnumEquality` (`.ChangeType` (break `StateTreeTransitionResult` Transition)) "Changed")
    (`AIController.K2_ClearFocus` (`self.Controller`))))
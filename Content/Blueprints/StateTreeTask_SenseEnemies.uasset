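; StateTree task that turns AI perception events into either a target enemy or an investigate location.
; It binds to perception updated and forgotten events while active, filtering sensed actors by tag.
; A forward-cone check plus visibility trace promotes a stimulus to the controller's target; otherwise, without a target, the strongest stimulus sets the investigate location.
; Forgetting the target, or any actor while untargeted, clears state and controller focus.
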(event `self.ReceiveLatentEnterState`
  (params (Transition :type "StateTreeTransitionResult Structure (by ref)"))
  (bind _aiperception (`/Game/Blueprints/BP_ShooterAIController.AIPerception` (`self.Controller`)))
  (if (`|EnumEquality` (`.ChangeType` (break `StateTreeTransitionResult` Transition)) "Changed")
    (add `AIPerceptionComponent.OnTargetPerceptionUpdated` _aiperception (`|CreateDelegate` :!event `On Perception Updated`))
    (add `AIPerceptionComponent.OnTargetPerceptionForgotten` _aiperception (`|CreateDelegate` :!event `On Perception Forgotten`))))

(event `self.ReceiveExitState`
  (params (Transition :type "StateTreeTransitionResult Structure (by ref)"))
  (bind _aiperception (`/Game/Blueprints/BP_ShooterAIController.AIPerception` (`self.Controller`)))
  (if (`|EnumEquality` (`.ChangeType` (break `StateTreeTransitionResult` Transition)) "Changed")
    (remove `AIPerceptionComponent.OnTargetPerceptionUpdated` _aiperception (`|CreateDelegate` :!event `On Perception Updated`))
    (remove `AIPerceptionComponent.OnTargetPerceptionForgotten` _aiperception (`|CreateDelegate` :!event `On Perception Forgotten`))))

(event `On Perception Updated`
  (params (Actor :type "Actor Object Reference") (Stimulus :type "AIStimulus Structure"))
  (bind (_age _expirationage _strength _stimuluslocation _receiverlocation _tag _bsuccessfullysensed) (break `AIStimulus` Stimulus))
  ; Does the sensed actor have the right tag? Have we successfully sensed it?
  (if (`Actor.ActorHasTag` Actor (`self.Sense Tag`))
    (if _bsuccessfullysensed
      ; Do we have direct line of sight to the stimulus causer?
      (bind _direct_line_of_sight (`self.Has Direct Line of Sight to Stimulus` _stimuluslocation Actor))
      (if _direct_line_of_sight
        ; We can see the target directly, so set it as a full sense and investigate it directly.
        (bind _output_get (set `self.Target Enemy` Actor))
        (`/Game/Blueprints/BP_ShooterAIController.Set Current Target` (`self.Controller`) _output_get)
        (set `self.Has Target` true)
        (set `self.Has Investigate Location` false)
        (else
          ; If we already have a direct target, ignore the partial stimulus and keep on the target.
          (if (not (`KismetSystemLibrary.IsValid` (`self.Target Enemy`)))
            ; Is this stimulus stronger than the last one we sensed?
            (if (> _strength (`self.Last Stimulus Strength`))
              ; Investigate the stimulus location instead.
              (set `self.Last Stimulus Strength` _strength)
              (set `self.Has Target` false)
              (set `self.Investigate Location` _stimuluslocation)
              (set `self.Has Investigate Location` true))))))))

(event `On Perception Forgotten`
  (params (Actor :type "Actor Object Reference"))
  (bind _target_enemy (`self.Target Enemy`))
  (bind _controller (`self.Controller`))
  ; Have we forgotten the current target?
  ; Are we forgetting about a partial sense?
  (if (== Actor _target_enemy)
    ; Clear the target data and flags
    (set `self.Target Enemy` null :!label _label)
    (set `self.Has Target` false)
    (set `self.Has Investigate Location` false)
    (set `self.Last Stimulus Strength` 0.0)
    ; Ensure the target data on the AI Controller is cleared too
    (`/Game/Blueprints/BP_ShooterAIController.Clear Current Target` _controller)
    (`AIController.K2_ClearFocus` _controller)
    (elif (not (`KismetSystemLibrary.IsValid` _target_enemy))
      (goto _label))))

(fn `Has Direct Line of Sight to Stimulus`
  (params (`Stimulus Locaiton` :type "Vector Structure") (`Stimulus Causer` :type "Actor Object Reference"))
  (returns (`Direct Line of Sight` :type Boolean))
  ; Is the stimulus in front of the character? If not, assume, it's not in direct line of sight.
  (if (>= (`KismetMathLibrary.Dot_VectorVector` (`KismetMathLibrary.Normal` (- `Stimulus Locaiton` (`Actor.K2_GetActorLocation` (`self.Character`)))) (`Actor.GetActorForwardVector` (`self.Character`))) (`KismetMathLibrary.DegCos` (`self.Direct Line of Sight Cone Angle`)))
    ; Run a line trace to the stimulus causer, ignoring both actors.
    ; If the trace is obstructed by anything else, assume there's no direct line of sight.
    (bind (_outhit _returnvalue) (`KismetSystemLibrary.LineTraceSingle` (`Actor.K2_GetActorLocation` (`self.Character`)) (`Actor.K2_GetActorLocation` (`local.Stimulus Causer`)) "TraceTypeQuery1" false (`|MakeArray` (`self.Character`) (`local.Stimulus Causer`) :!type "Actor Object Reference")))
    (return (not _returnvalue))
    (else
      (return false))))
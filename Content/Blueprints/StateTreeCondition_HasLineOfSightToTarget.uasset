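; StateTree condition that tests whether a Character has, or lacks, line of sight to a Target, with MustHaveLineOfSight selecting the expected result.
; An invalid target or one outside the facing cone counts as no line of sight.
; Otherwise, visibility traces run from the first-person camera to evenly spaced heights on the target's colliding bounds, ignoring the target.
; The first unobstructed trace counts as line of sight.
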(fn `ReceiveGetDescription`
  (params (Formatting :type "EStateTreeNodeFormatting Enum" :default "RichText"))
  (returns (ReturnValue :type Text))
  (return (`KismetMathLibrary.SelectText` "<b>HAS</b> Line of Sight to Target" "Has <b>NO</b> Line of Sight to Target" (`self.Must Have Line of Sight`))))

(fn `ReceiveTestCondition`
  (returns (ReturnValue :type Boolean))
  (locals (`Target Center of Mass` :type "Vector Structure") (`Target Half Extent Z` :type "Float (double-precision)") (`Target Extent Z Offset` :type "Float (double-precision)"))
  (bind (_origin _boxextent) (`Actor.GetActorBounds` (`self.Target`) true false))
  (`|ExecutionSequence`
    (:`then_0`
      ; Skip tests if the target has been destroyed already
      (if (not (`KismetSystemLibrary.IsValid` (`self.Target`)))
        (return (not (`self.Must Have Line of Sight`)))))
    (:`then_1`
      ; Check if the character is facing the target enough that they could theoretically shoot it.
      (if (not (>= (`KismetMathLibrary.Dot_VectorVector` (`KismetMathLibrary.GetDirectionUnitVector` (`Actor.K2_GetActorLocation` (`self.Character`)) (`Actor.K2_GetActorLocation` (`self.Target`))) (`Actor.GetActorForwardVector` (`self.Character`))) (`KismetMathLibrary.DegCos` (`self.Line of Sight Cone Angle`))))
        (return (not (`self.Must Have Line of Sight`)))))
    (:`then_2`
      ; Extract data from the target's bounding box, so we can run a number of line traces at various heights to determine if we have unobstructed line of sight.
      (set `local.Target Center of Mass` _origin)
      (bind _output_get (set `local.Target Half Extent Z` (.z _boxextent)))
      (set `local.Target Extent Z Offset` (/ (* _output_get 2.0) (`self.Number of Vertical Line of Sight Checks`)))
      ; Split the target bounding box into N vertical segment traces
      (for _index (range (`self.Number of Vertical Line of Sight Checks`))
        ; Run a visibility trace to the target at the current height offset. Ignore the character and target, so as soon as we find an unobstructed trace we know we have LoS
        (bind (_outhit _returnvalue) (`KismetSystemLibrary.LineTraceSingle` (`SceneComponent.K2_GetComponentLocation` (`/Game/Blueprints/BP_FirstPersonCharacter.FirstPersonCamera` (`self.Character`))) (+ (`local.Target Center of Mass`) (`KismetMathLibrary.MakeVector` 0.0 0.0 (- (`local.Target Half Extent Z`) (* _index (`local.Target Extent Z Offset`))))) "TraceTypeQuery1" false (`|MakeArray` (`self.Target`))))
        (if (not _returnvalue)
          (return (`self.Must Have Line of Sight`)))))
    (:`then_3`
      ; All test traces were obstructed, so we don't have line of sight
      (return (not (`self.Must Have Line of Sight`))))))